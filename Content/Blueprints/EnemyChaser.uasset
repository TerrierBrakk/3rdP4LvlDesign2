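; Enemy chaser pawn that pursues a TopViewPlayer spotted by PawnSensing, using AIMoveTo and dealing damage on arrival, then re-chasing after a short delay.
; AnyDamage lowers Health, then subtracts Damage again for an exact-zero test that destroys the actor, otherwise printing the instigator's name.
; A looping Patrol event alternates between two target points with pauses, but nothing in this graph calls it.
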(event OnSeePawn(PawnSensing)
  (params (Pawn :type Pawn%20Object%20Reference))
  ;[1 1 1] Seguimos al jugador cuando vemos al pawn
  (bind _astop_view_player (Utilities|Casting|CastToTopViewPlayer Pawn))
  (CallFunction|ChasePlayer _astop_view_player))

(event Custom|Patrol
  (AI|AIMoveTo self "0.000000, 0, 0" (Variables|Default|GetTargetPoint1) 5.0 false
    (:OnSuccess
      (Utilities|FlowControl|Delay 3.0)
      (AI|AIMoveTo self "0, 0, 0" (Variables|Default|GetTargetPoint2) 5.0 false
        (:OnSuccess
          (Utilities|FlowControl|Delay 3.0)
          (CallFunction|Patrol))))))

(event Custom|ChasePlayer
  (params (PlayerToChase :type Actor%20Object%20Reference))
  ;[1 1 1] Chase Action
  (AI|AIMoveTo self "0, 0, 0" PlayerToChase 5.0 false
    (:OnSuccess
      (Game|Damage|ApplyDamage PlayerToChase (Math|Conversions|ToFloat(Integer) (Variables|Default|GetDamage%20dealt)) 0 0)
      (Utilities|FlowControl|Delay 1.0)
      (CallFunction|ChasePlayer PlayerToChase))))

(event EventBeginPlay)

(event Game|Damage|EventAnyDamage
  (params (Damage :type Float%20%28single-precision%29) (DamageType :type Damage%20Type%20Object%20Reference) (InstigatedBy :type Controller%20Object%20Reference) (DamageCauser :type Actor%20Object%20Reference))
  ;[1 1 1] Recibe cualquier dañi
  (Variables|Default|SetHealth (Math|Float|Truncate (- (Math|Conversions|ToFloat(Integer) (Variables|Default|GetHealth)) Damage)))
  (if (== (- (Math|Conversions|ToFloat(Integer) (Variables|Default|GetHealth)) Damage) 0.0)
    (Actor|DestroyActor)
    (else
      (Development|PrintString (Utilities|GetDisplayName InstigatedBy)))))

(fn ConstructionScript)