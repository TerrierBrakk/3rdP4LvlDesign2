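; Enemy AI character that roams, patrols or chases, starting from its IAState on BeginPlay.
; Each behavior is a self-repeating AIMoveTo loop: random navigable points nearby, cycling PatrolPoints, or following a target and applying damage on arrival.
; PawnSensing switches it to chasing a seen TopViewPlayer, with a one-time alert sound.
; Incoming damage lowers Health, plays a hit sound and destroys the actor when Health minus Damage, subtracted again, reaches zero.
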(event OnSeePawn(PawnSensing)
  (params (Pawn :type Pawn%20Object%20Reference))
  ;[1 1 1] Sigue al jugador cuando lo ve
  (bind _astop_view_player (Utilities|Casting|CastToTopViewPlayer Pawn))
  (Development|PrintString "DETECTADO" true true "(R=0.562500,G=0.057845,B=0.000000,A=1.000000)" 1.0)
  (Utilities|FlowControl|Sequence
    (:then_0
      (CallFunction|Chasing _astop_view_player))
    (:then_1
      (Utilities|FlowControl|DoOnce false
        (:Completed
          (Audio|PlaySoundatLocation "/Game/Sounds/SFX/GuardVoice_-_Alert.GuardVoice_-_Alert" (Transformation|GetActorLocation) "0, 0, 0" 1.0 1.0 0.0 0 0 0))))))

(event Custom|Patrol
  ;[1 1 1] Patrullaje entre 2 puntos
  (AI|AIMoveTo self "0, 0, 0" (Utilities|Array|Get(acopy) (Variables|Default|GetPatrolPoints) (Variables|Default|GetTargetPointIndex)) 5.0 false
    (:OnSuccess
      (Utilities|FlowControl|Delay (Variables|Default|GetDelayWaitPatrol))
      (if (>= (Variables|Default|GetTargetPointIndex) (- (Utilities|Array|Length (Variables|Default|GetPatrolPoints)) 1))
        (Variables|Default|SetTargetPointIndex 0)
        (else
          (Math|Integer|IncrementInt (Variables|Default|GetTargetPointIndex)
            (:%20%20
              _))))
      (CallFunction|Patrol))))

(event Custom|Chasing
  (params (Player%20to%20chase :type Actor%20Object%20Reference))
  ;[1 1 1] Seguir al Jugador
  (AI|AIMoveTo self "0, 0, 0" Player%20to%20chase 2.0 false
    (:OnSuccess
      (Game|Damage|ApplyDamage Player%20to%20chase (Math|Conversions|ToFloat(Integer) (Variables|Default|GetDaño)) 0 0)
      (Utilities|FlowControl|Delay 1.0)
      (CallFunction|Chasing Player%20to%20chase))))

(event Custom|MoveToRandomLoc
  ;[1 1 1] Agarra su Ubicacion y camina random en un radio de 500 m
  (AI|AIMoveTo self (.RandomLocation (Class|NavigationSystemV1|GetRandomPointinNavigableRadius (Transformation|GetActorLocation) 5e+02 0 0)) 0 5.0 false
    (:OnSuccess
      (Utilities|FlowControl|Delay 2.0)
      (CallFunction|MovetoRandomLoc))))

(event EventBeginPlay
  ;[1 1 1] Estados de mi IA
  (switch Utilities|FlowControl|Switch|SwitchonIAState (Variables|Default|GetIAState)
    (:NewEnumerator1
      (CallFunction|MovetoRandomLoc))
    (:NewEnumerator2
      (CallFunction|Chasing))
    (:NewEnumerator3
      (CallFunction|Patrol))))

(event Game|Damage|EventAnyDamage
  (params (Damage :type Float%20%28single-precision%29) (DamageType :type Damage%20Type%20Object%20Reference) (InstigatedBy :type Controller%20Object%20Reference) (DamageCauser :type Actor%20Object%20Reference))
  ;[1 1 1] Recibo daño
  (bind _output_get (Variables|Default|SetHealth (Math|Float|Truncate (- (Math|Conversions|ToFloat(Integer) (Variables|Default|GetHealth)) Damage))))
  (Audio|PlaySoundatLocation "/Game/Sounds/SFX/DanoEnemigo.DanoEnemigo" (Transformation|GetActorLocation) "0, 0, 0" 1.0 1.0 0.0 0 0 0)
  (Development|PrintString (Utilities|String|ToString(Integer) _output_get) true true "(R=0.996072,G=0.076200,B=1.000000,A=1.000000)")
  (if (<= (- (Math|Conversions|ToFloat(Integer) (Variables|Default|GetHealth)) Damage) 0.0)
    (Actor|DestroyActor)
    (else
      (Development|PrintString (Utilities|GetDisplayName InstigatedBy)))))

(fn ConstructionScript)